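; Player character for a side-scrolling platformer with health, coins, checkpoints, dash and barrel cannons.
; Enhanced Input drives X-axis movement, jump and a timed, gravity-free dash with cooldown.
; Entering a barrel hides the character and removes movement input until it fires along the barrel's arrow; landing or bouncing restores gravity and controls.
; Damage grants brief invulnerability; respawning returns to the checkpoint at a life's cost, and zero life reloads the level.
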(event Custom|TerminarDash
  (if (Variables|Propiedades|GetbPuedeDisparar?)
    (Variables|Propiedades|SetbEstaDasheando? false)
    (else
      (Variables|/Script/Engine.MovementComponent|SetVelocity (Variables|Character|GetCharacterMovement) "0, 0, 0")
      (Variables|Propiedades|SetbEstaDasheando? false)
      (Variables|/Script/Engine.CharacterMovementComponent|SetGravityScale (Variables|Character|GetCharacterMovement) 2.0)))
  (Utilities|Time|ClearTimerbyFunctionName 0 "TerminarDash"))

(event Input|EnhancedActionEvents|EnhancedInputActionIA_Movimiento
  (params (ActionValue :type Float%20%28double-precision%29) (ElapsedSeconds :type Float%20%28double-precision%29) (TriggeredSeconds :type Float%20%28double-precision%29) (InputAction :type Input%20Action%20Object%20Reference :default "/Game/Inputs/InputAction/IA_Movimiento.IA_Movimiento"))
  (bind _returnvalue (Pawn|GetController))
  (Pawn|Input|AddMovementInput "1.000000,0.000000,0.000000" ActionValue false)
  (Math|Float|CompareFloat (.x (Pawn|Components|CharacterMovement|GetCurrentAcceleration (Variables|Character|GetCharacterMovement))) 0.0
    (:>
      (Pawn|SetControlRotation _returnvalue (Math|Rotator|MakeRotator 0.0 0.0 0.0)))
    (:<
      (Pawn|SetControlRotation _returnvalue (Math|Rotator|MakeRotator 0.0 0.0 1.8e+02)))))

(event Input|EnhancedActionEvents|EnhancedInputActionIA_Salto
  (params (ActionValue :type Boolean) (ElapsedSeconds :type Float%20%28double-precision%29) (TriggeredSeconds :type Float%20%28double-precision%29) (InputAction :type Input%20Action%20Object%20Reference :default "/Game/Inputs/InputAction/IA_Salto.IA_Salto"))
  (:Triggered
    (Character|Jump))
  (:Completed
    (Character|StopJumping)))

(event Input|EnhancedActionEvents|EnhancedInputActionIA_Dash
  (params (ActionValue :type Boolean) (ElapsedSeconds :type Float%20%28double-precision%29) (TriggeredSeconds :type Float%20%28double-precision%29) (InputAction :type Input%20Action%20Object%20Reference :default "/Game/Inputs/InputAction/IA_Dash.IA_Dash"))
  (:Started
    (if (Variables|Propiedades|GetbPuedeHacerDash?)
      (Variables|Propiedades|SetbPuedeHacerDash? false)
      (Variables|/Script/Engine.CharacterMovementComponent|SetGravityScale (Variables|Character|GetCharacterMovement) 0.0)
      (Variables|Propiedades|SetbEstaDasheando? true)
      (Character|LaunchCharacter (* (Transformation|GetActorForwardVector) (Variables|Propiedades|GetVelocidadDash)) true true)
      (Utilities|Time|SetTimerbyEvent (delegate Custom|TerminarDash) (Variables|Propiedades|GetDuracionDash))
      (Utilities|FlowControl|Delay (Variables|Propiedades|GetTiempoParaVolverHacerDash))
      (Variables|Propiedades|SetbPuedeHacerDash? true))))

(event Input|EnhancedActionEvents|EnhancedInputActionIA_Salir
  (params (ActionValue :type Boolean) (ElapsedSeconds :type Float%20%28double-precision%29) (TriggeredSeconds :type Float%20%28double-precision%29) (InputAction :type Input%20Action%20Object%20Reference :default "/Game/Inputs/InputAction/IA_Salir.IA_Salir"))
  (Game|QuitGame 0 "Quit" false))

(event Input|EnhancedActionEvents|EnhancedInputActionIA_Disparar
  (params (ActionValue :type Boolean) (ElapsedSeconds :type Float%20%28double-precision%29) (TriggeredSeconds :type Float%20%28double-precision%29) (InputAction :type Input%20Action%20Object%20Reference :default "/Game/Inputs/InputAction/IA_Disparar.IA_Disparar"))
  (bind _returnvalue (Pawn|GetController))
  (if (Variables|Propiedades|GetbPuedeDisparar?)
    (Pawn|Components|CharacterMovement|SetMovementMode (Variables|Character|GetCharacterMovement) "MOVE_Walking" 0)
    (Transformation|DetachFromActor "KeepWorld" "KeepWorld" "KeepWorld")
    (Character|LaunchCharacter (* (Math|Vector|GetForwardVector (Actor|GetComponentbyClass (Variables|Propiedades|GetBarrilReferencia) "/Script/Engine.ArrowComponent")) (Variables|Propiedades|GetVelocidadDash)) true true)
    (Rendering|SetActorHiddenInGame false)
    (Audio|PlaySound2D "/Game/Sounds/392995__josecruz98__disparo-canon.392995__josecruz98__disparo-canon" 1.0 1.0 0.0 0 0)
    (Transformation|SetActorRotation "0, 0, 0")
    (if (> (.pitch (Transformation|GetWorldRotation (Variables|/Script/Engine.Actor|GetRootComponent (Variables|Propiedades|GetBarrilReferencia)))) 0.0)
      (Pawn|SetControlRotation _returnvalue (Math|Rotator|MakeRotator 0.0 0.0 1.8e+02))
      (else
        (Pawn|SetControlRotation _returnvalue (Math|Rotator|MakeRotator 0.0 0.0 0.0))))
    (Variables|Propiedades|SetbPuedeDisparar? false)))

(event EventBeginPlay
  (bind _asplayer_controller (Utilities|Casting|CastToPlayerController (Pawn|GetController)))
  (Input|AddMappingContext (PlayerController|LocalPlayerSubsystems|GetEnhancedInputLocalPlayerSubsystem _asplayer_controller) "/Game/Inputs/MappingContext/IMC_PersonajeInputs.IMC_PersonajeInputs" 0 "(bIgnoreAllPressedKeysUntilRelease=True,bForceImmediately=False,bNotifyUserSettings=False)")
  (Input|AddMappingContext (PlayerController|LocalPlayerSubsystems|GetEnhancedInputLocalPlayerSubsystem _asplayer_controller) "/Game/Inputs/MappingContext/IMC_Barril.IMC_Barril" 0 "(bIgnoreAllPressedKeysUntilRelease=True,bForceImmediately=False,bNotifyUserSettings=False)"))

(event EventActualizarCheckpoint
  (params (CheckpointAlcanzado :type Vector :default "0, 0, 0"))
  (Variables|Propiedades|SetZonaSegura CheckpointAlcanzado))

(event EventObtenerMonedas
  (params (Monedas :type Integer))
  (Variables|Mochila|SetMonedas (+ Monedas (Variables|Mochila|GetMonedas))))

(event EventRespawnear
  (bind _charactermovement (Variables|Character|GetCharacterMovement))
  (Components|Movement|StopMovementImmediately _charactermovement)
  (Variables|/Script/Engine.MovementComponent|SetVelocity _charactermovement "0, 0, 0")
  (CallFunction|RestaurarControles)
  (CallFunction|RestarVida)
  (Transformation|SetActorLocation (Variables|Propiedades|GetZonaSegura) false false))

(event EventEntrarBarril
  (params (Barril :type BP%20Barril%20Object%20Reference))
  (Variables|Propiedades|SetbEstaDasheando? false)
  (Variables|Propiedades|SetBarrilReferencia Barril)
  (Rendering|SetActorHiddenInGame true)
  (Components|Movement|StopMovementImmediately (Variables|Character|GetCharacterMovement))
  (Variables|Propiedades|SetbPuedeDisparar? true)
  (if (Variables|/Game/2D/Sprites/object/BP_Barril.BP_Barril_C|GetbEsMovil? (Variables|Propiedades|GetBarrilReferencia))
    (Transformation|AttachActorToActor (Variables|Propiedades|GetBarrilReferencia) "None" "KeepRelative" "KeepRelative" "KeepRelative" true))
  (Transformation|SetActorLocation (Transformation|GetActorLocation (Variables|Propiedades|GetBarrilReferencia)) false false)
  (Variables|/Script/Engine.CharacterMovementComponent|SetGravityScale (Variables|Character|GetCharacterMovement) 0.0)
  (bind _asplayer_controller (Utilities|Casting|CastToPlayerController (Pawn|GetController)))
  (Input|RemoveMappingContext (PlayerController|LocalPlayerSubsystems|GetEnhancedInputLocalPlayerSubsystem _asplayer_controller) "/Game/Inputs/MappingContext/IMC_PersonajeInputs.IMC_PersonajeInputs" "(bIgnoreAllPressedKeysUntilRelease=True,bForceImmediately=False,bNotifyUserSettings=False)"))

(event EventOnLanded
  (params (Hit :type Hit%20Result%20Structure%20%28by%20ref%29))
  (CallFunction|RestaurarControles))

(event EventPossessed
  (params (NewController :type Controller%20Object%20Reference))
  (bind _returnvalue (UserInterface|CreateWidget "/Game/UI/WP_BarraSalud.WP_BarraSalud_C" (Game|GetPlayerController 0)))
  (Actor|SetOwner 0)
  (UserInterface|Viewport|AddtoViewport _returnvalue 0))

(event EventDañar
  (params (PosicionEnemigo :type Vector :default "0, 0, 0"))
  (if (not (Variables|Propiedades|GetbEstaDañado?))
    (CallFunction|RestarVida)
    (Variables|Propiedades|SetbEstaDañado? true)
    (Utilities|FlowControl|Delay 1.0)
    (Variables|Propiedades|SetbEstaDañado? false)))

(event EventRebotar
  (CallFunction|RestaurarControles)
  (Character|LaunchCharacter "0.000000,0.000000,1000.000000" true true))

(fn ConstructionScript)

(fn ReiniciarNivel
  (bind _returnvalue (Game|GetCurrentLevelName true))
  (Game|OpenLevel(byName) (Utilities|String|StringToName _returnvalue)))

(fn RestaurarControles
  (Variables|/Script/Engine.CharacterMovementComponent|SetGravityScale (Variables|Character|GetCharacterMovement) 2.0)
  (bind _asplayer_controller (Utilities|Casting|CastToPlayerController (Pawn|GetController)))
  (Input|AddMappingContext (PlayerController|LocalPlayerSubsystems|GetEnhancedInputLocalPlayerSubsystem _asplayer_controller) "/Game/Inputs/MappingContext/IMC_PersonajeInputs.IMC_PersonajeInputs" 0 "(bIgnoreAllPressedKeysUntilRelease=True,bForceImmediately=False,bNotifyUserSettings=False)"))

(fn RestarVida
  (bind _output_get (Variables|Propiedades|SetVida (- (Variables|Propiedades|GetVida) 1.0)))
  (if (== _output_get 0.0)
    (CallFunction|ReiniciarNivel)))