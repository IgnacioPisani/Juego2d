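; Bat enemy for the 2D game that moves along a fixed pattern and damages the player on contact.
; On BeginPlay it stores its location as a center, then flags select a timeline-driven circular, vertical or reversed vertical motion.
; The circle offsets the center by the forward vector of an animated pitch scaled by Radio.
; Capsule overlap with BP_Personaje sends it a Dañar message with the bat's location.
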(event OnComponentBeginOverlap(CapsuleComponent)
  (params (OverlappedComponent :type Primitive%20Component%20Object%20Reference) (OtherActor :type Actor%20Object%20Reference) (OtherComp :type Primitive%20Component%20Object%20Reference) (OtherBodyIndex :type Integer) (bFromSweep :type Boolean) (SweepResult :type Hit%20Result%20Structure%20%28by%20ref%29))
  (Utilities|Casting|CastToBP_Personaje OtherActor)
  (Class|BPIDañar|Dañar(Message) OtherActor (Transformation|GetActorLocation)))

(event EventBeginPlay
  (Variables|Propiedades|SetCentro (Transformation|GetActorLocation))
  (if (Variables|Propiedades|GetEsCircular?)
    (bind _newtrack_0 (Timeline|MovimientoCircular PlayFromStart)
      (:Update
        (Transformation|SetActorLocation (+ (* (Math|Vector|GetForwardVector (Math|Rotator|MakeRotator 0.0 _newtrack_0 0.0)) (Variables|Propiedades|GetRadio)) (Variables|Propiedades|GetCentro)) false false)))
    (elif (Variables|Propiedades|GetEsLineal?)
      (bind _newtrack_0_2 (Timeline|MovimientoLineal PlayFromStart)
        (:Update
          (Transformation|SetActorLocation (+ (Math|Vector|MakeVector 0.0 0.0 _newtrack_0_2) (Variables|Propiedades|GetCentro)) false false)))
      (elif (Variables|Propiedades|GetEsLinealInverso?)
        (Timeline|MovimientoLineal ReverseFromEnd)))))

(event Collision|EventActorBeginOverlap
  (params (OtherActor :type Actor%20Object%20Reference)))

(event EventTick
  (params (DeltaSeconds :type Float%20%28single-precision%29)))

(fn ConstructionScript)