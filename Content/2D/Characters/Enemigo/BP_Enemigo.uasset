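; BP_Enemigo is a patrolling enemy for a 2D game that hurts BP_Personaje and can be stomped.
; MoverAdelante moves it forward if SeMueve is set, and wall or ledge detectors turn it around.
; DamageDetector starts repeating damage on contact, while DeadDetector hides it, disables collision and bounces the player.
; Rather than being destroyed, it returns at its start position through the bound ZonaPincho OnRespawn event.
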(event OnComponentBeginOverlap(DeadDetector)
  (params (OverlappedComponent :type Primitive%20Component%20Object%20Reference) (OtherActor :type Actor%20Object%20Reference) (OtherComp :type Primitive%20Component%20Object%20Reference) (OtherBodyIndex :type Integer) (bFromSweep :type Boolean) (SweepResult :type Hit%20Result%20Structure%20%28by%20ref%29))
  (Utilities|Casting|CastToBP_Personaje OtherActor)
  (Audio|PlaySound2D "/Game/Sounds/177848__motion_s__modulated-ruler-fx-spring-jump-cartoon-noise.177848__motion_s__modulated-ruler-fx-spring-jump-cartoon-noise" 1.0 1.0 0.0 0 0)
  (Rendering|SetActorHiddenInGame true)
  (Collision|SetActorEnableCollision false)
  (Class|BPIRebotar|Rebotar(Message) OtherActor))

(event OnComponentBeginOverlap(WallDetector)
  (params (OverlappedComponent :type Primitive%20Component%20Object%20Reference) (OtherActor :type Actor%20Object%20Reference) (OtherComp :type Primitive%20Component%20Object%20Reference) (OtherBodyIndex :type Integer) (bFromSweep :type Boolean) (SweepResult :type Hit%20Result%20Structure%20%28by%20ref%29))
  (CallFunction|RotarEnemigo))

(event OnComponentEndOverlap(LedgeDetector)
  (params (OverlappedComponent :type Primitive%20Component%20Object%20Reference) (OtherActor :type Actor%20Object%20Reference) (OtherComp :type Primitive%20Component%20Object%20Reference) (OtherBodyIndex :type Integer))
  (CallFunction|RotarEnemigo))

(event OnComponentBeginOverlap(DamageDetector)
  (params (OverlappedComponent :type Primitive%20Component%20Object%20Reference) (OtherActor :type Actor%20Object%20Reference) (OtherComp :type Primitive%20Component%20Object%20Reference) (OtherBodyIndex :type Integer) (bFromSweep :type Boolean) (SweepResult :type Hit%20Result%20Structure%20%28by%20ref%29))
  (Utilities|Casting|CastToBP_Personaje OtherActor)
  (Class|BPIDañar|Dañar(Message) OtherActor (Transformation|GetActorLocation))
  (Utilities|Time|SetTimerbyEvent (delegate Custom|SeguirDañando) 0.5 true))

(event OnComponentEndOverlap(DamageDetector)
  (params (OverlappedComponent :type Primitive%20Component%20Object%20Reference) (OtherActor :type Actor%20Object%20Reference) (OtherComp :type Primitive%20Component%20Object%20Reference) (OtherBodyIndex :type Integer))
  (Utilities|Time|ClearTimerbyFunctionName 0 "SeguirDañando"))

(event Custom|MoverAdelante
  (if (Variables|Propiedades|GetbSeMueve?)
    (Pawn|Input|AddMovementInput (Transformation|GetActorForwardVector) (Variables|Propiedades|GetVelocidad) false)))

(event Custom|Bind
  (EventDispatchers|BindEventtoOnRespawn (Variables|Propiedades|GetZonaPincho) (delegate Custom|RestaurarEnemigo)))

(event Custom|SeguirDañando
  (Class|BPIDañar|Dañar(Message) (stale OnComponentBeginOverlap(DamageDetector) OtherActor) (Transformation|GetActorLocation)))

(event Custom|RestaurarEnemigo
  (Rendering|SetActorHiddenInGame false)
  (Collision|SetActorEnableCollision true)
  (Transformation|SetActorLocation (Variables|Propiedades|GetPosicionInicial) false false))

(event EventBeginPlay
  (Variables|Propiedades|SetPosicionInicial (Transformation|GetActorLocation)))

(fn ConstructionScript)

(fn RotarEnemigo
  (if (Variables|Propiedades|GetbSeMueve?)
    (Transformation|SetActorRotation (Math|Rotator|CombineRotators (Transformation|GetActorRotation) "0.000000,180.000000,0.000000"))))

(fn SetearZonaPinchos
  (params (ZonaPincho :type BP%20Pincho%20Collider%20Object%20Reference))
  (Variables|Propiedades|SetZonaPincho ZonaPincho))