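; Barrel actor for a 2D game that captures overlapping actors implementing BPI_EntrarBarril by sending them an enter-barrel message.
; On entry, a rotator barrel steps its pitch through four angles on a looping timer; otherwise a mobile one ping-pongs along X via a reversing timeline.
; Resetear, which Bind hooks to the spike zone's respawn event, restores initial rotation and angle index and stops the timeline.
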(event OnComponentBeginOverlap(Box)
  (params (OverlappedComponent :type Primitive%20Component%20Object%20Reference) (OtherActor :type Actor%20Object%20Reference) (OtherComp :type Primitive%20Component%20Object%20Reference) (OtherBodyIndex :type Integer) (bFromSweep :type Boolean) (SweepResult :type Hit%20Result%20Structure%20%28by%20ref%29))
  (if (Utilities|DoesObjectImplementInterface OtherActor "/Game/2D/Interfaces/BPI_EntrarBarril.BPI_EntrarBarril_C")
    (Variables|Propiedades|SetbEstaEnElBarril? true)
    (Class|BPIEntrarBarril|EntrarBarril(Message) OtherActor self)
    (if (Variables|Propiedades|GetbEsRotador?)
      (Utilities|Time|SetTimerbyEvent (delegate Custom|RotarBarril) 0.5 true)
      (elif (Variables|Propiedades|GetbEsMovil?)
        (CallFunction|MovementBarrilForward)))))

(event OnComponentEndOverlap(Box)
  (params (OverlappedComponent :type Primitive%20Component%20Object%20Reference) (OtherActor :type Actor%20Object%20Reference) (OtherComp :type Primitive%20Component%20Object%20Reference) (OtherBodyIndex :type Integer))
  (Utilities|Time|ClearTimerbyFunctionName 0 "RotarBarril")
  (Variables|Propiedades|SetbEstaEnElBarril? false))

(event Custom|Bind
  (EventDispatchers|BindEventtoOnRespawn (Variables|Propiedades|GetZonaPinchos) (delegate Custom|Resetear)))

(event Custom|Resetear
  (Transformation|SetActorRotation (Variables|Propiedades|GetRotacion))
  (Variables|Propiedades|SetAngulosIndex 0)
  (Utilities|FlowControl|Sequence
    (:then_0
      (bind (_direction _linealbarrel) (Timeline|Timeline_0 Stop)
        (:Update
          (Transformation|SetRelativeLocation (Variables|Default|GetBox) (Math|Vector|MakeVector (.x (+ (Variables|Propiedades|GetUbicacionInicial) (Math|Vector|MakeVector (* _linealbarrel (Variables|Propiedades|GetMultiplicadorMovimiento)) 0.0 0.0))) (.y (+ (Variables|Propiedades|GetUbicacionInicial) (Math|Vector|MakeVector (* _linealbarrel (Variables|Propiedades|GetMultiplicadorMovimiento)) 0.0 0.0))) (.z (+ (Variables|Propiedades|GetUbicacionInicial) (Math|Vector|MakeVector (* _linealbarrel (Variables|Propiedades|GetMultiplicadorMovimiento)) 0.0 0.0)))) false false))
        (:Finished
          (switch Utilities|FlowControl|Switch|SwitchonETimelineDirection _direction
            (:Forward
              (CallFunction|MovementBarrilBack))
            (:Backward
              (CallFunction|MovementBarrilForward))))))
    (:then_1
      (Timeline|Timeline_0 SetNewTime))))

(event Custom|RotarBarril
  (bind _angulosindex (Variables|Propiedades|GetAngulosIndex))
  (Transformation|SetRelativeRotation (Variables|Default|GetBox) (Math|Rotator|MakeRotator 0.0 (+ (Utilities|Array|Get(acopy) (Variables|Propiedades|GetAngulos) _angulosindex) (.pitch (Variables|Propiedades|GetRotacion))) 0.0) false false)
  (CallFunction|CalcularIndexAngulo _angulosindex))

(event Custom|MovementBarrilForward
  (bind (_direction _linealbarrel) (Timeline|Timeline_0 Play)
    (:Update
      (Transformation|SetRelativeLocation (Variables|Default|GetBox) (Math|Vector|MakeVector (.x (+ (Variables|Propiedades|GetUbicacionInicial) (Math|Vector|MakeVector (* _linealbarrel (Variables|Propiedades|GetMultiplicadorMovimiento)) 0.0 0.0))) (.y (+ (Variables|Propiedades|GetUbicacionInicial) (Math|Vector|MakeVector (* _linealbarrel (Variables|Propiedades|GetMultiplicadorMovimiento)) 0.0 0.0))) (.z (+ (Variables|Propiedades|GetUbicacionInicial) (Math|Vector|MakeVector (* _linealbarrel (Variables|Propiedades|GetMultiplicadorMovimiento)) 0.0 0.0)))) false false))
    (:Finished
      (switch Utilities|FlowControl|Switch|SwitchonETimelineDirection _direction
        (:Forward
          (CallFunction|MovementBarrilBack))
        (:Backward
          (CallFunction|MovementBarrilForward))))))

(event Custom|MovementBarrilBack
  (bind (_direction _linealbarrel) (Timeline|Timeline_0 Reverse)
    (:Update
      (Transformation|SetRelativeLocation (Variables|Default|GetBox) (Math|Vector|MakeVector (.x (+ (Variables|Propiedades|GetUbicacionInicial) (Math|Vector|MakeVector (* _linealbarrel (Variables|Propiedades|GetMultiplicadorMovimiento)) 0.0 0.0))) (.y (+ (Variables|Propiedades|GetUbicacionInicial) (Math|Vector|MakeVector (* _linealbarrel (Variables|Propiedades|GetMultiplicadorMovimiento)) 0.0 0.0))) (.z (+ (Variables|Propiedades|GetUbicacionInicial) (Math|Vector|MakeVector (* _linealbarrel (Variables|Propiedades|GetMultiplicadorMovimiento)) 0.0 0.0)))) false false))
    (:Finished
      (switch Utilities|FlowControl|Switch|SwitchonETimelineDirection _direction
        (:Forward
          (CallFunction|MovementBarrilBack))
        (:Backward
          (CallFunction|MovementBarrilForward))))))

(event EventBeginPlay
  (Variables|Propiedades|SetUbicacionInicial (Transformation|GetActorLocation))
  (Variables|Propiedades|SetRotacion (Transformation|GetActorRotation)))

(fn ConstructionScript)

(fn CalcularIndexAngulo
  (params (Index :type Integer))
  (Variables|Propiedades|SetAngulosIndex (Math|Integer|%(Integer) (+ Index 1) 4)))

(fn GetRotacion
  (return (Variables|Propiedades|GetRotacion)))

(fn SetearZonaPinchos
  (params (ZonaPinchos :type BP%20Pincho%20Collider%20Object%20Reference))
  (Variables|Propiedades|SetZonaPinchos ZonaPinchos))