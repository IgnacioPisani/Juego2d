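; A 2D collapsing platform that disappears after the player steps on it and returns on respawn.
; A Box overlap with BP_Personaje starts a TiempoCaida timer that hides the actor and disables its PaperSprite collision.
; A spike zone reference is set through SetearZonaPinchos.
; The Bind event hooks that zone's OnRespawn to Resetear, which restores visibility and collision without recreating the actor.
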(event OnComponentBeginOverlap(Box)
  (params (OverlappedComponent :type Primitive%20Component%20Object%20Reference) (OtherActor :type Actor%20Object%20Reference) (OtherComp :type Primitive%20Component%20Object%20Reference) (OtherBodyIndex :type Integer) (bFromSweep :type Boolean) (SweepResult :type Hit%20Result%20Structure%20%28by%20ref%29))
  (Utilities|Casting|CastToBP_Personaje OtherActor)
  (Utilities|Time|SetTimerbyEvent (delegate Custom|Eliminar%20Plataforma) (Variables|Propiedades|GetTiempoCaida)))

(event Custom|Bind
  (EventDispatchers|BindEventtoOnRespawn (Variables|Propiedades|GetZonaPinchos) (delegate Custom|Resetear)))

(event Custom|Resetear
  (Rendering|SetActorHiddenInGame false)
  (Collision|SetCollisionEnabled (Variables|Default|GetPaperSprite) "QueryAndPhysics"))

(event Custom|Eliminar%20Plataforma
  (Rendering|SetActorHiddenInGame true)
  (Collision|SetCollisionEnabled (Variables|Default|GetPaperSprite) "NoCollision"))

(event EventBeginPlay)

(event Collision|EventActorBeginOverlap
  (params (OtherActor :type Actor%20Object%20Reference)))

(event EventTick
  (params (DeltaSeconds :type Float%20%28single-precision%29)))

(fn ConstructionScript)

(fn SetearZonaPinchos
  (params (ZonaPinchos :type BP%20Pincho%20Collider%20Object%20Reference))
  (Variables|Propiedades|SetZonaPinchos ZonaPinchos))