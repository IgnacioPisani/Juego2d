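; BP_PinchoCollider is a spike hazard collider that respawns actors touching its box.
; On BeginPlay it registers itself with every BP_PlataformaDerrumbable (collapsible platform) and calls Bind on each.
; On overlap, actors implementing BPI_ActualizarCheckpoint receive RespawnearMessage, then the OnRespawn dispatcher fires, giving bound listeners such as the platforms a respawn signal.
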(event OnComponentBeginOverlap(Box)
  (params (OverlappedComponent :type Primitive%20Component%20Object%20Reference) (OtherActor :type Actor%20Object%20Reference) (OtherComp :type Primitive%20Component%20Object%20Reference) (OtherBodyIndex :type Integer) (bFromSweep :type Boolean) (SweepResult :type Hit%20Result%20Structure%20%28by%20ref%29))
  (if (Utilities|DoesObjectImplementInterface OtherActor "/Game/2D/Interfaces/BPI_ActualizarCheckpoint.BPI_ActualizarCheckpoint_C")
    (Class|BPIRespawnear|Respawnear(Message) OtherActor)
    (Default|CallOnRespawn)))

(event EventBeginPlay
  (bind _outactors (Actor|GetAllActorsOfClass "/Game/2D/Sprites/object/BP_PlataformaDerrumbable.BP_PlataformaDerrumbable_C"))
  (for _array_element _outactors
    (Utilities|IsValid _array_element
      (:Is%20Valid
        (Default|SetearZonaPinchos _array_element self)
        (Default|Bind _array_element)))))

(event Collision|EventActorBeginOverlap
  (params (OtherActor :type Actor%20Object%20Reference)))

(event EventTick
  (params (DeltaSeconds :type Float%20%28single-precision%29)))

(fn ConstructionScript)